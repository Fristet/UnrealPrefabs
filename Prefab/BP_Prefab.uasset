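; BP_Prefab is a data-driven prefab that rebuilds a group of static meshes from PrefabDataTable.
; Its construction script adds one component per row, setting the mesh, transform and materials.
; It then overrides relative rotation by parsing the Transform column's string, feeding the rotation's raw X, Y and Z directly into roll, pitch and yaw without quaternion conversion.
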(fn `UserConstructionScript`
  (bind _prefab_datatable (`self.Prefab_DataTable`))
  (bind _outrownames (`DataTableFunctionLibrary.GetDataTableRowNames` _prefab_datatable))
  (for (_array_element _array_index) _outrownames
    (bind _returnvalue (`|GetDataTableRow` _prefab_datatable _array_element)
      (:`then`
        (bind (_staticmesh _materials _transform) (break `/Game/Prefab/ST_Prefab_Single` _returnvalue))
        (bind _returnvalue_2 (`AddComponent|NODE_AddStaticMeshComponent-1` :`RelativeTransform` _transform))
        (`StaticMeshComponent.SetStaticMesh` _returnvalue_2 _staticmesh)
        (bind _returnvalue_3 (`DataTableFunctionLibrary.GetDataTableColumnAsString` _prefab_datatable "Transform"))
        (bind _outconvertedvector (`KismetStringLibrary.Conv_StringToVector` (`.RightS` (`KismetStringLibrary.Split` (`KismetStringLibrary.Split` (`|GetArrayItem` _returnvalue_3 _array_index) ",W") "=("))))
        (`SceneComponent.K2_SetRelativeRotation` _returnvalue_2 (`KismetMathLibrary.MakeRotator` (.x _outconvertedvector) (.y _outconvertedvector) (.z _outconvertedvector)) false false)
        (for (_array_element_2 _array_index_2) _materials
          (`PrimitiveComponent.SetMaterial` _returnvalue_2 _array_index_2 _array_element_2))))))